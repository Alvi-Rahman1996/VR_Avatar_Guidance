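; BP_Avatar1 is a lobby avatar Blueprint for Basic Multiplayer with AI movement and a debug-style spawn toggle.
; MoveAvatarTo runs AIMoveTo toward a given location and prints the result, leaving its speed inputs unused.
; The 2 key alternates between spawning another BP_Avatar1 at a hardcoded position and destroying the actor in NewVar.
; The spawned avatar is never stored in this instance's NewVar, so the destroy step does not target it.
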(event Custom|Move%20Avatar%20To
  (params (Location :type Vector) (Speed :type Float%20%28double-precision%29) (Normal%20Speed :type Float%20%28double-precision%29))
  (bind _movementresult (AI|AIMoveTo self Location 0 5.0 false)
    (:then
      (Development|PrintString (Utilities|String|EnumtoString _movementresult)))
    (:OnSuccess
      (Development|PrintString "All Done!"))
    (:OnFail
      (Development|PrintString "Failed to move!"))))

(event Input|KeyboardEvents|2
  (params (Key :type Key%20Structure :default "None"))
  (:Pressed
    (Utilities|FlowControl|FlipFlop
      (:A
        (bind _returnvalue (Game|SpawnActorfromClass "BP_Avatar1_C" (Math|Conversions|ToTransform(Vector) (Math|Vector|MakeVector 7.2e+02 3e+01 88.0)) "Undefined" "MultiplyWithRoot" 0 0))
        (Variables|BP_Avatar1_C|SetNewVar _returnvalue 0))
      (:B
        (Actor|DestroyActor (Variables|Default|GetNewVar))))))

(fn ConstructionScript)