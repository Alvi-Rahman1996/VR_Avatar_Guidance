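; Base multiplayer GameMode that tracks connected player controllers and provides player spawning.
; PostLogin and controller swaps add controllers to AllPCs, and logout removes those that cast to BP_PC_BaseSetup.
; SpawnPlayer destroys any pawn the controller holds, then spawns a BP_ThirdPersonCharacter at a randomly picked player start and possesses it.
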(event EventBeginPlay)

(event EventTick
  (params (DeltaSeconds :type Float%20%28single-precision%29)))

(event EventPostLogin
  (params (NewPlayer :type Player%20Controller%20Object%20Reference))
  ;[1 1 1] Comment
  (Utilities|Array|Add (Variables|Default|GetAll_PCs) NewPlayer))

(event EventOnSwapPlayerControllers
  (params (OldPC :type Player%20Controller%20Object%20Reference) (NewPC :type Player%20Controller%20Object%20Reference))
  ;[1 1 1] Comment
  (Utilities|Array|Add (Variables|Default|GetAll_PCs) NewPC))

(event EventOnLogout
  (params (ExitingController :type Controller%20Object%20Reference))
  ;[1 1 1] Comment
  (bind _asbp_pc_base_setup (Utilities|Casting|CastToBP_PC_BaseSetup ExitingController))
  (Utilities|Array|RemoveItem (Variables|Default|GetAll_PCs) _asbp_pc_base_setup))

(fn ConstructionScript)

(fn FindRandomPlayerStart
  (bind _outactors (Actor|GetAllActorsOfClass 0))
  (return (Transformation|GetActorTransform (Utilities|Array|Get(acopy) _outactors (Math|Random|RandomIntegerinRange 0 (+ (Utilities|Array|Length _outactors) -1))))))

(fn SpawnPlayer
  (params (PlayerController :type Player%20Controller%20Object%20Reference))
  (bind _returnvalue (Pawn|GetControlledPawn PlayerController))
  (Utilities|IsValid _returnvalue
    (:Is%20Valid
      (Actor|DestroyActor _returnvalue))
    (:Is%20Not%20Valid
      _))
  (bind _returnvalue_2 (Game|SpawnActorfromClass "/Game/ThirdPerson/Blueprints/BP_ThirdPersonCharacter.BP_ThirdPersonCharacter_C" (Spawning|FindRandomPlayerStart) "Undefined" "MultiplyWithRoot" 0 0))
  (Pawn|Possess PlayerController _returnvalue_2))